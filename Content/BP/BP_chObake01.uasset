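; BP_chObake01 is a ghost (obake) enemy that displays its enemy number and animates at random intervals.
; On BeginPlay it writes TekiBango to a text render component, then enters an endless delay loop.
; After each random short wait, it plays one of three montages on its mesh's anim instance: CrMont or its right (Migi) and left (Hidari) variants.
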(event `self.ReceiveBeginPlay`
  (`TextRenderComponent.K2_SetText` (`self.TextRender`) (`KismetTextLibrary.Conv_IntToText` (`self.tekiBango`)))
  (`KismetSystemLibrary.Delay` (`KismetMathLibrary.RandomFloatInRange` 1.0 2.0) :!label _label)
  (`AnimInstance.Montage_Play` (`SkeletalMeshComponent.GetAnimInstance` (`self.Mesh`)) (select `int` (`KismetMathLibrary.RandomIntegerInRange` 0 2) :`0` (`self. crMont`) :`1` (`self. crMont_migi`) :`2` (`self. crMont_hidari`)) 1.0 "MontageLength" 0.0 true)
  (goto _label))

(fn `UserConstructionScript`)