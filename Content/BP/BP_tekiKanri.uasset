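; BP_tekiKanri is an enemy manager that spawns BP_chObake01 characters inside its Box volume, up to five in total.
; Each TekiMake call spawns one at a random point in the box, passes Bangou as its TekiBango index and gives it a default controller.
; It then increments Bangou and appends the enemy to ObakeAly.
; Bangou never decreases here, so once the cap is reached further calls only print a message.
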(event `/Game/BP/BPI_kanriMess.tekiMake`
  (if (> (`self.bangou`) 4)
    (`KismetSystemLibrary.PrintString` "MAX 5")
    (else
      (bind _returnvalue (`|SpawnActorFromClass` "/Game/BP/BP_chObake01.BP_chObake01_C" (`KismetMathLibrary.Conv_VectorToTransform` (`KismetMathLibrary.RandomPointInBoundingBox` (`self.K2_GetActorLocation`) (`BoxComponent.BoxExtent` (`self.Box`)))) "AdjustIfPossibleButAlwaysSpawn" "OverrideRootScale" null (`self.bangou`) null))
      (`Pawn.SpawnDefaultController` _returnvalue)
      (set `self.bangou` (+ (`self.bangou`) 1))
      (`KismetArrayLibrary.Array_Add` (`self.obakeAly`) _returnvalue))))

(fn `UserConstructionScript`)